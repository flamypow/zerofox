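; BP_Ship is the player ship, sliding its body in a bounded plane to follow the aim position from the gameplay UI.
; Each Tick, math expressions map the UI's X and Y aim ratios between bounds to relative Y and Z, keeping depth and rotation fixed.
; MoveComponentTo moves ShipBody there over distance divided by Speed, for constant-speed travel.
; A getter exposes the GameplayUI reference; BeginPlay and Possessed are empty.
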(event EventBeginPlay)

(event EventTick
  (params (DeltaSeconds :type Float%20%28single-precision%29))
  (bind _gameplay_ui (Variables|Default|GetGameplay%20UI))
  (bind _shipbody (Variables|Default|GetShipBody))
  (bind _result (Math|Float|NegateFloat (|(((RightBound-LeftBound)*Ratio)+LeftBound) (Variables|Default|GetRightBoundY) (Variables|Default|GetLeftBoundY) (Variables|/Game/AMainGameMechanics/UI_InGame.UI_InGame_C|GetShipAimYRatio _gameplay_ui)))
    (:%20%20
      (Components|MoveComponentTo _shipbody (Math|Vector|MakeVector (.x (Variables|/Script/Engine.SceneComponent|GetRelativeLocation (Variables|Default|GetShipBody))) (|(((RightBound-LeftBound)*Ratio)+LeftBound) (Variables|Default|GetRightBoundX) (Variables|Default|GetLeftBoundX) (Variables|/Game/AMainGameMechanics/UI_InGame.UI_InGame_C|GetShipAimXRatio _gameplay_ui)) _result) (Variables|/Script/Engine.SceneComponent|GetRelativeRotation _shipbody) false false (/ (Math|Vector|VectorLength (- (Math|Vector|MakeVector (.x (Variables|/Script/Engine.SceneComponent|GetRelativeLocation (Variables|Default|GetShipBody))) (|(((RightBound-LeftBound)*Ratio)+LeftBound) (Variables|Default|GetRightBoundX) (Variables|Default|GetLeftBoundX) (Variables|/Game/AMainGameMechanics/UI_InGame.UI_InGame_C|GetShipAimXRatio _gameplay_ui)) _result) (Variables|/Script/Engine.SceneComponent|GetRelativeLocation (Variables|Default|GetShipBody)))) (Variables|Default|GetSpeed)) false))))

(event EventPossessed
  (params (NewController :type Controller%20Object%20Reference)))

(fn ConstructionScript)

(fn GetGamePlayUI
  (return (Variables|Default|GetGameplay%20UI)))