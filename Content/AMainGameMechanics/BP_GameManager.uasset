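; Game manager that runs a dwell-to-complete check on the ship's aim for the fire icon.
; Each Tick copies aim ratios from UIWidget and, while FireIconState is zero, times how long ShipAimWithInCenter holds, resetting when it fails.
; Once TimeToCompleteFire elapses, it turns the icon off through the widget; TurnFireIconOn is exposed but not called here.
; The FireBoxBound center-box test in ShipAimWithInCenter appears unconnected.
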(event `self.ReceiveBeginPlay`)

(event `self.ReceiveTick`
  (params (DeltaSeconds :type "Float (single-precision)"))
  (bind _uiwidget (`self.UIWidget`))
  (set `self.ShipAimXRatio` (`/Game/AMainGameMechanics/UI_InGame.ShipAimXRatio` _uiwidget))
  (set `self.ShipAimYRatio` (`/Game/AMainGameMechanics/UI_InGame.ShipAimYRatio` _uiwidget))
  (if (== (`/Game/AMainGameMechanics/UI_InGame.FireIconState` (`self.UIWidget`)) 0)
    (if (`self.ShipAimWithInCenter`)
      (if (!= (`self.CurrentTimeCharged`) 0.0)
        (if (> (- (`GameplayStatics.GetTimeSeconds`) (`self.CurrentTimeCharged`)) (`self.TimeToCompleteFire`))
          (`self.TurnFireIconOff`))
        (else
          (set `self.CurrentTimeCharged` (`GameplayStatics.GetTimeSeconds`))))
      (else
        (set `self.CurrentTimeCharged` 0.0)))))

(fn `TurnFireIconOff`
  (`/Game/AMainGameMechanics/UI_InGame.TurnFireIconOff` (`self.UIWidget`)))

(fn `TurnFireIconOn`
  (`/Game/AMainGameMechanics/UI_InGame.TurnFireIconOn` (`self.UIWidget`)))

(fn `UserConstructionScript`)