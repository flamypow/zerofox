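; BP_BaseEnemy is an enemy actor that registers itself as a lock-on target when the ship's aim is over it.
; BeginPlay caches BP_GameManager, and Tick projects the Widget's world location into viewport ratios to compare against the manager's ship aim ratios.
; Within a small tolerance on both axes, it shows the Widget, turns on the fire icon and adds itself to the lock-on list.
; Nothing here hides the Widget again.
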(event `self.ReceiveBeginPlay`
  (bind _returnvalue (`GameplayStatics.GetActorOfClass` "/Game/AMainGameMechanics/BP_GameManager.BP_GameManager_C"))
  (set `self.GameManager` _returnvalue))

(event `self.ReceiveTick`
  (params (DeltaSeconds :type "Float (single-precision)"))
  (bind _gamemanager (`self.GameManager`))
  (bind _gamemanager_2 (`self.GameManager`))
  (bind (_returnvalue_x _returnvalue_y) (`KismetMathLibrary.BreakVector2D` (/ (`PlayerController.ProjectWorldLocationToScreen` (`GameplayStatics.GetPlayerController` 0) (`SceneComponent.K2_GetComponentLocation` (`self.Widget`)) false) (`WidgetLayoutLibrary.GetViewportSize`))))
  (bind _returnvalue (- _returnvalue_x (`/Game/AMainGameMechanics/BP_GameManager.ShipAimXRatio` _gamemanager_2)))
  (bind _returnvalue_2 (- _returnvalue_y (`/Game/AMainGameMechanics/BP_GameManager.ShipAimYRatio` _gamemanager_2)))
  (if (and (and (< _returnvalue 0.05) (> _returnvalue -0.05)) (and (< _returnvalue_2 0.05) (> _returnvalue_2 -0.05)))
    (`SceneComponent.SetVisibility` (`self.Widget`) true false)
    (`/Game/AMainGameMechanics/BP_GameManager.TurnFireIconOn` _gamemanager)
    (`/Game/AMainGameMechanics/BP_GameManager.AddToLockOnList` _gamemanager self)))

(fn `UserConstructionScript`)